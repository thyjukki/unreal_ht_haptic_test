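; Locomotive car Blueprint for the hands train example, handling smoke, whistle and starting or stopping.
; Events activate the billow particles with their audio and play the whistle sound.
; AnimateStartStop lerps CurrentSpeed to a goal by re-calling itself after a zero-second Delay each frame, rather than using Tick or a Timeline.
; On completion it sets IsMoving, then either plays the engine sound or deactivates the smoke particles.
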(event `self.ReceiveBeginPlay`)

(event `self.BlowLotsOfSmoke`
  ;[1 1 1] Smoke billow effect
  (`ActorComponent.Activate` (`self.BillowParticleSystem`) true)
  (`AudioComponent.Play` (`self.BillowAudio`) 0.0))

(event `self.WhistleButtonStateChanged`
  ;[1 1 1] Whistle event
  (`AudioComponent.Play` (`self.WhistleAudio`) 0.0))

(event `self.AnimateStartStop`
  (params (bStartTrain :type Boolean) (StartSpeed :type "Float (single-precision)") (GoalSpeed :type "Float (single-precision)") (SpeedChangeDuration :type "Float (single-precision)") (SpeedChangeTimeLeft :type "Float (single-precision)"))
  ;[1 1 1] Start/Stop Train
  (if (<= SpeedChangeTimeLeft 0.0)
    (set `self.CurrentSpeed` GoalSpeed :!label _label)
    (bind _output_get (set `self.bIsMoving` bStartTrain))
    (if _output_get
      (`self.PlayEngineSoundAndGetLength` "AccelerateOrSetProperSpeed")
      (else
        (`ActorComponent.Deactivate` (`self.SmokeParticleSystem`))))
    (set `self.bIsStartingOrStopping` false)
    (elif (`KismetMathLibrary.NearlyEqual_FloatFloat` (`self.CurrentSpeed`) GoalSpeed)
      (goto _label)
      (else
        (set `self.CurrentSpeed` (`KismetMathLibrary.Lerp` StartSpeed GoalSpeed (`KismetMathLibrary.FClamp` (/ (- SpeedChangeDuration SpeedChangeTimeLeft) SpeedChangeDuration))))
        (set `self.NextSpeedChangeTimeLeft` (`KismetMathLibrary.FClamp` (- SpeedChangeTimeLeft (`GameplayStatics.GetWorldDeltaSeconds`)) 0.0 SpeedChangeTimeLeft))
        (`KismetSystemLibrary.Delay` 0.0)
        (`self.AnimateStartStop` bStartTrain StartSpeed GoalSpeed SpeedChangeDuration (`self.NextSpeedChangeTimeLeft`))))))

(fn `UserConstructionScript`)