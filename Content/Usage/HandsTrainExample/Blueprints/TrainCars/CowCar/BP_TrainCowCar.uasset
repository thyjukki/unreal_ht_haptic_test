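; BP_TrainCowCar is a train car in the hands train example that carries a cow, which hops and moos when triggered.
; The GoMooCowGo event plays the CowHop timeline from the start and starts the moo audio.
; Each timeline update drives the cow body's relative location and rotation, plus separate rotations for the head and tail.
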(event `self.ReceiveBeginPlay`)

(event `self.GoMooCowGo`
  (bind _cow (`self.Cow`))
  (bind _mooaudio (`self.MooAudio`))
  ;[1 1 1] Animate Cow hop
  (`|ExecutionSequence`
    (:`then_0`
      (bind (_direction _maincowposition _maincowrotation _cowheadrotation _cowtailrotation) (`Timeline|CowHop` :!via `PlayFromStart`)
        (:`Update`
          (`|ExecutionSequence`
            (:`then_0`
              (`SceneComponent.K2_SetRelativeLocation` _cow _maincowposition false false))
            (:`then_1`
              (`SceneComponent.K2_SetRelativeRotation` _cow (`KismetMathLibrary.MakeRotator` (.x _maincowrotation) (.y _maincowrotation) (.z _maincowrotation)) false false))
            (:`then_2`
              (`SceneComponent.K2_SetRelativeRotation` (`self.Cow_Head`) (`KismetMathLibrary.MakeRotator` (.x _cowheadrotation) (.y _cowheadrotation) (.z _cowheadrotation)) false false))
            (:`then_3`
              (`SceneComponent.K2_SetRelativeRotation` (`self.Cow_Tail`) (`KismetMathLibrary.MakeRotator` (.x _cowtailrotation) (.y _cowtailrotation) (.z _cowtailrotation)) false false))))))
    (:`then_1`
      (`ActorComponent.SetActive` _mooaudio true false)
      (`AudioComponent.Play` _mooaudio 0.0))))

(fn `UserConstructionScript`)