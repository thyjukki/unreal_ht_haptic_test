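; BP_ControllerBox is a near-field interactable actor in the HandsTrain example that can glide to a target location.
; LerptoPosition re-calls itself each frame through a zero-second Delay, using CalculateTimedLerp to turn remaining time into a clamped alpha.
; It lerps from the current location rather than StartPosition, so it moves faster than linear.
; On arrival or timeout it snaps to the end and clears IsLerpingToHMD.
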(event `self.LerpToPosition`
  (params (LerpTotalDuration :type "Float (single-precision)") (TimeLeftForLerp :type "Float (single-precision)") (StartPosition :type "Vector Structure") (EndPosition :type "Vector Structure"))
  (bind _returnvalue (`self.K2_GetActorLocation`))
  ;[1 1 1] Lerp actor to position
  (if (<= TimeLeftForLerp 0.0)
    (set `self.bIsLerpingToHMD` false :!label _label)
    (`self.K2_SetActorLocation` EndPosition)
    (elif (== EndPosition _returnvalue)
      (goto _label)
      (else
        (bind _lerpvalue (`self.CalculateTimedLerp` LerpTotalDuration TimeLeftForLerp))
        (`self.K2_SetActorLocation` (`KismetMathLibrary.VLerp` _returnvalue EndPosition _lerpvalue))
        (bind _output_get (set `self.NextTimeLeft` (- TimeLeftForLerp (`GameplayStatics.GetWorldDeltaSeconds`))))
        (`KismetSystemLibrary.Delay` 0.0)
        (`self.LerpToPosition` LerpTotalDuration _output_get StartPosition EndPosition)))))

(fn `CalculateTimedLerp`
  (params (TotalTime :type "Float (double-precision)") (TimeLeft :type "Float (double-precision)"))
  (returns (LerpValue :type "Float (double-precision)"))
  (return (`KismetMathLibrary.FClamp` (/ (- TotalTime TimeLeft) TotalTime))))

(fn `UserConstructionScript`)