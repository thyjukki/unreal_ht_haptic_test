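; Hands visualization switcher for the HandsTrainExample scene that locates the player's Oculus hand components and initializes meshes from them.
; FindBothHands polls until hand tracking is enabled and a HandsTrainExamplePawn exists, retrying through Delay loops.
; FindHandsOnPawn scans the pawn root's child components and stores RightHand and LeftHand by skeleton type, then InitializeMeshesFromHands runs, defined outside these graphs.
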(event `self.FindBothHands`
  ;[1 1 1] Wait until hand tracking is enabled
  (if (`OculusInputFunctionLibrary.IsHandTrackingEnabled`) :!label _label
    ;[1 1 1] Find Pawn
    (bind _returnvalue (`GameplayStatics.GetActorOfClass` "/Game/Usage/HandsTrainExample/Blueprints/HandsTrainExamplePawn.HandsTrainExamplePawn_C" :!label _label_2))
    (if (`KismetSystemLibrary.IsValid` _returnvalue)
      (`self.FindHandsOnPawn` _returnvalue)
      (`self.InitializeMeshesFromHands`)
      (else
        (`KismetSystemLibrary.Delay` 0.0)
        (goto _label_2)))
    (else
      (`KismetSystemLibrary.Delay` 0.2)
      (goto _label))))

(fn `FindHandsOnPawn`
  (params (Pawn :type "Actor Object Reference"))
  (for _array_element (`SceneComponent.GetChildrenComponents` (`Actor.RootComponent` Pawn) true)
    (bind _asoculus_hand_component (cast `OculusHandComponent` _array_element))
    (`|ExecutionSequence`
      (:`then_0`
        (bind _skeletontype (`OculusHandComponent.SkeletonType` _asoculus_hand_component))
        (if (`|EnumEquality` _skeletontype "HandRight")
          (set `self.RightHand` _asoculus_hand_component)))
      (:`then_1`
        (if (`|EnumEquality` _skeletontype "HandLeft")
          (set `self.LeftHand` _asoculus_hand_component))))))

(fn `UserConstructionScript`)