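; Windmill actor for the HandsTrain example's far-field items that manages blade speed and matching audio, starting in the moving state at BeginPlay.
; NewMoveState toggles motion, calling the start or stop sound sequence and ramping CurrentSpeed toward maximum or zero.
; ChangeSpeed interpolates linearly by re-calling itself each frame through a zero Delay, avoiding Tick.
; Timed delays chain the start sound into a fast or slow loop chosen by MaxBladesSpeed.
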(event `self.ReceiveBeginPlay`
  (`self.NewMoveState` true))

(event `self.NewMoveState`
  (params (IsMovingNow :type Boolean))
  (bind _bladesaudio (`self.BladesAudio`))
  (bind _bladesaudio_2 (`self.BladesAudio`))
  ;[1 1 1] Move State Event
  (set `self.IsMoving` IsMovingNow)
  (`ActorComponent.Activate` (`self.BladesAudio`) false)
  (if IsMovingNow
    (`|ExecutionSequence`
      (:`then_0`
        (`AudioComponent.Stop` _bladesaudio_2)
        (`AudioComponent.SetSound` _bladesaudio_2 "/Game/Usage/HandsTrainExample/Audio/S_WindmillStart.S_WindmillStart")
        (`AudioComponent.Play` _bladesaudio_2 0.0)
        (`KismetSystemLibrary.Delay` 1.9)
        (if (> (`self.MaxBladesSpeed`) 150.0)
          (`AudioComponent.SetSound` _bladesaudio_2 "/Game/Usage/HandsTrainExample/Audio/S_WindmillRotateFastLoop.S_WindmillRotateFastLoop")
          (else
            (`AudioComponent.SetSound` _bladesaudio_2 "/Game/Usage/HandsTrainExample/Audio/S_WindmillRotateSlowLoop.S_WindmillRotateSlowLoop")))
        (`AudioComponent.Play` _bladesaudio_2 0.0))
      (:`then_1`
        (`self.ChangeSpeed` 3.0 3.0 (`self.CurrentSpeed`) (`self.MaxBladesSpeed`))))
    (else
      (`|ExecutionSequence`
        (:`then_0`
          (`AudioComponent.SetSound` _bladesaudio "/Game/Usage/HandsTrainExample/Audio/S_WindmillStop.S_WindmillStop")
          (`AudioComponent.Play` _bladesaudio 0.0)
          (`KismetSystemLibrary.Delay` 1.74)
          (`AudioComponent.Stop` _bladesaudio))
        (:`then_1`
          (`self.ChangeSpeed` 3.0 3.0 (`self.CurrentSpeed`)))))))

(event `self.ChangeSpeed`
  (params (SpeedChangeDuration :type "Float (single-precision)") (TimeLeftForSpeedChange :type "Float (single-precision)") (StartSpeed :type "Float (single-precision)") (TargetSpeed :type "Float (single-precision)"))
  ;[1 1 1] Change Speed Event
  (bind _output_get (set `self.CurrentSpeed` (`KismetMathLibrary.Lerp` StartSpeed TargetSpeed (`KismetMathLibrary.FClamp` (/ (- SpeedChangeDuration TimeLeftForSpeedChange) SpeedChangeDuration)))))
  (if (not (`KismetMathLibrary.NearlyEqual_FloatFloat` _output_get TargetSpeed))
    (bind _output_get_2 (set `self.NextTimeLeftChangeDur` (- TimeLeftForSpeedChange (`GameplayStatics.GetWorldDeltaSeconds`))))
    (`KismetSystemLibrary.Delay` 0.0)
    (`self.ChangeSpeed` SpeedChangeDuration _output_get_2 StartSpeed TargetSpeed)))

(fn `UserConstructionScript`)