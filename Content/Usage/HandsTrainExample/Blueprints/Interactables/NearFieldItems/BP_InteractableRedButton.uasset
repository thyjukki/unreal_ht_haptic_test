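; Interactable red button for the hand-tracking example that triggers glove haptics when touched.
; On BeginPlay it binds a contact-zone event, which on Enter picks the right or left glove address from the touching tool and sends an async HTTP haptic request.
; Separate events, not called within this Blueprint, lerp the button mesh back to its saved position by re-invoking themselves each frame, or stop that reset.
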(event `self.ReceiveBeginPlay`
  (add `Interactable.OnContactZoneEvent` (delegate `OnContactZoneEvent_Event_0`)))

(event `OnContactZoneEvent_Event_0`
  (params (ColliderArgs :type "ColliderZoneArgs Structure (by ref)"))
  (bind (_zone _collisionframe _collidingtool _interactiont) (break `ColliderZoneArgs` ColliderArgs))
  (if (`|EnumEquality` _interactiont "Enter")
    (`KismetSystemLibrary.PrintString` "Triggering touch")
    (if (`InteractableTool.IsRightHandedTool` _collidingtool)
      (bind _returnvalue (`GloveTestLibrary.GetGloveAddress` "Right"))
      (`KismetSystemLibrary.PrintString` _returnvalue)
      (`LZAsyncAction_RequestHttpMessage.AsyncRequestHTTP` _returnvalue 12 200 5 120 1)
      (else
        (bind _returnvalue_2 (`GloveTestLibrary.GetGloveAddress` "Left"))
        (`KismetSystemLibrary.PrintString` _returnvalue_2)
        (`LZAsyncAction_RequestHttpMessage.AsyncRequestHTTP` _returnvalue_2 13 200 5 120 1)))))

(event `self.StopResetLerp`
  (`self.ResetPositionLerp` 0.0) ; By calling this function, we stop any previous lerp. Make duration 0 because we just want to stop.
)

(event `self.ResetPositionLerp`
  (params (ResetDuration :type "Float (single-precision)") (TimeLeftForReset :type "Float (single-precision)"))
  (bind _buttonmeshcomp (`self.ButtonMeshComp`))
  ;[1 1 1] Position Reset Logic
  (if (== (`ButtonMeshHelper.OldRelativePosition` (`self.ButtonMeshHelper`)) (`SceneComponent.RelativeLocation` (`self.ButtonMeshComp`)))
    _
    (elif (<= TimeLeftForReset 0.0)
      _
      (elif (not (`KismetMathLibrary.NearlyEqual_FloatFloat` ResetDuration))
        (bind _lerpvalue (`self.CalculateLerpFromDuration` ResetDuration TimeLeftForReset))
        (`SceneComponent.K2_SetRelativeLocation` _buttonmeshcomp (`KismetMathLibrary.VLerp` (`SceneComponent.RelativeLocation` _buttonmeshcomp) (`ButtonMeshHelper.OldRelativePosition` (`self.ButtonMeshHelper`)) _lerpvalue) false false)
        (bind _output_get (set `self.NextTimeLeftVal` (`KismetMathLibrary.FMax` (- TimeLeftForReset (`GameplayStatics.GetWorldDeltaSeconds`)))))
        (`KismetSystemLibrary.Delay` 0.0)
        (`self.ResetPositionLerp` ResetDuration _output_get)))))

(fn `CalculateLerpFromDuration`
  (params (TotalDuration :type "Float (double-precision)") (TimeLeft :type "Float (double-precision)"))
  (returns (LerpValue :type "Float (double-precision)"))
  (return (`KismetMathLibrary.FClamp` (/ (- TotalDuration TimeLeft) TotalDuration))))

(fn `UserConstructionScript`)