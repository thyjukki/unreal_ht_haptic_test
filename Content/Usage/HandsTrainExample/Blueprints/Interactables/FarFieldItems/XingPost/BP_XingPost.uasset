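; Railroad crossing post for the HandsTrainExample that alternately blinks its two warning light surfaces for a set duration.
; BlinkLights re-calls itself each frame through zero-second Delays, counting down blink and animation time and flipping which light leads at each interval.
; AffectLightColors cross-fades the TintAlpha material parameter between the two surfaces.
; When animation time runs out, the lights are toggled off via ToggleLightObjects.
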(event `self.ReceiveBeginPlay`)

(event `self.BlinkLights`
  (params (TimeLeftUntilNextBlink :type "Float (single-precision)") (LightBlinkDuration :type "Float (single-precision)") (TimeLeftForAnimation :type "Float (single-precision)"))
  (bind _returnvalue (`GameplayStatics.GetWorldDeltaSeconds`))
  (bind _returnvalue_2 (- TimeLeftForAnimation _returnvalue))
  ;[1 1 1] Blink Lights Event
  (if (> TimeLeftForAnimation 0.0)
    (`self.AffectLightColors` TimeLeftUntilNextBlink LightBlinkDuration)
    (if (<= TimeLeftUntilNextBlink 0.0)
      (set `self.BlinkFirstLight` (not (`self.BlinkFirstLight`)))
      (`KismetSystemLibrary.Delay` 0.0)
      (`self.BlinkLights` LightBlinkDuration LightBlinkDuration _returnvalue_2)
      (else
        (`KismetSystemLibrary.Delay` 0.0)
        (`self.BlinkLights` (- TimeLeftUntilNextBlink _returnvalue) LightBlinkDuration _returnvalue_2)))
    (else
      (`self.ToggleLightObjects` false))))

(fn `AffectLightColors`
  (params (TimeLeftUntilNextBlink :type "Float (double-precision)") (BlinkDuration :type "Float (double-precision)"))
  (bind _returnvalue (/ (- BlinkDuration TimeLeftUntilNextBlink) BlinkDuration))
  (bind _returnvalue_2 (- 1.0 (`KismetMathLibrary.FClamp` _returnvalue)))
  (if (`self.BlinkFirstLight`)
    (`MeshComponent.SetScalarParameterValueOnMaterials` (`self.LightSurface1`) "TintAlpha" _returnvalue)
    (`MeshComponent.SetScalarParameterValueOnMaterials` (`self.LightSurface2`) "TintAlpha" _returnvalue_2)
    (else
      (`MeshComponent.SetScalarParameterValueOnMaterials` (`self.LightSurface2`) "TintAlpha" _returnvalue)
      (`MeshComponent.SetScalarParameterValueOnMaterials` (`self.LightSurface1`) "TintAlpha" _returnvalue_2))))

(fn `UserConstructionScript`)