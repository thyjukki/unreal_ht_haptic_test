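; Manager actor for the HandsTrain example that spawns interactable hand tools and attaches their logic to the pawn's tracked Oculus hands.
; On BeginPlay it polls with delays until hand tracking is enabled, the HandsTrainExamplePawn exists and hand collision capsules are found.
; InitializeToolsOnPawn then spawns each class in LeftHandTools or RightHandTools by skeleton type and links it to its hand through AssociateToolWithHand.
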(event `self.ReceiveBeginPlay`
  ;[1 1 1] Wait until hand tracking has been turned on
  (if (`OculusInputFunctionLibrary.IsHandTrackingEnabled`) :!label _label
    ;[1 1 1] FindPawn
    (bind _returnvalue (`GameplayStatics.GetActorOfClass` "/Game/Usage/HandsTrainExample/Blueprints/HandsTrainExamplePawn.HandsTrainExamplePawn_C" :!label _label_2))
    (if (`KismetSystemLibrary.IsValid` _returnvalue)
      (bind _rootcomponent (`Actor.RootComponent` _returnvalue))
      (for _array_element (`SceneComponent.GetChildrenComponents` _rootcomponent true) :!label _label_3
        (bind _asoculus_hand_component (cast `OculusHandComponent` _array_element))
        (if (not (> (`KismetArrayLibrary.Array_Length` (`OculusHandComponent.CollisionCapsules` _asoculus_hand_component)) 0))
          (`KismetSystemLibrary.Delay` 0.2) ; Try to find capsules after soem delay if we failed
          (goto _label_3)))
      (`self.InitializeToolsOnPawn` _rootcomponent)
      (else
        (`KismetSystemLibrary.Delay` 0.0)
        (goto _label_2)))
    (else
      (`KismetSystemLibrary.Delay` 0.2)
      (goto _label))))

(fn `InitializeToolsOnPawn`
  (params (Pawn :type "SceneComponent Object Reference"))
  (bind _returnvalue (`self.GetTransform`))
  (for _array_element (`SceneComponent.GetChildrenComponents` Pawn true)
    (bind _asoculus_hand_component (cast `OculusHandComponent` _array_element))
    (if (`|EnumEquality` (`OculusHandComponent.SkeletonType` _asoculus_hand_component) "HandLeft")
      (for _array_element_2 (`self.LeftHandTools`)
        (bind _returnvalue_2 (`|SpawnActorFromClass` _array_element_2 _returnvalue "Undefined" "OverrideRootScale" null null))
        (`self.AssociateToolWithHand` _asoculus_hand_component _returnvalue_2))
      (else
        (for _array_element_3 (`self.RightHandTools`)
          (bind _returnvalue_3 (`|SpawnActorFromClass` _array_element_3 _returnvalue "Undefined" "OverrideRootScale" null null))
          (`self.AssociateToolWithHand` _asoculus_hand_component _returnvalue_3))))))

(fn `UserConstructionScript`)